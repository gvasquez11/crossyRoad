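; Player chicken character that hops in fixed grid steps along four directions.
; Each directional press adds an audio component; release rotates the mesh, calls Jump, instantly offsets the actor one step and re-applies the camera's current transform.
; IsJumping is set and cleared within the same release, so it does not span the jump.
; Tick re-enables input and adds zero movement; helper functions are empty.
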(event `self.ReceiveTick`
  (params (DeltaSeconds :type "Float (single-precision)"))
  (`self.EnableInput` null)
  (`self.AddMovementInput` (0.0 0.0 0.0)))

(event `InputAction|Left`
  (params (Key :type "Key Structure"))
  (bind (_returnvalue_x _returnvalue_y _returnvalue_z) (`KismetMathLibrary.BreakVector` (`self.K2_GetActorLocation`)))
  (bind (_returnvalue_x_2 _returnvalue_y_2 _returnvalue_z_2) (`KismetMathLibrary.BreakVector` (`SceneComponent.K2_GetComponentLocation` (`self.Camera`))))
  (:`Pressed`
    (`AddComponent|NODE_AddAudioComponent-10`))
  (:`Released`
    (if (not (`self.isJumping`))
      (`SceneComponent.K2_SetRelativeRotation` (`self.Mesh`) (struct :`Yaw` 270.0) false false)
      (set `self.isJumping` true)
      (`self.Jump`)
      (`self.K2_SetActorRelativeLocation` (`KismetMathLibrary.MakeVector` _returnvalue_x (+ _returnvalue_y -215.0) _returnvalue_z))
      (`SceneComponent.K2_SetWorldLocationAndRotation` (`self.Camera`) (`KismetMathLibrary.MakeVector` _returnvalue_x_2 _returnvalue_y_2 _returnvalue_z_2) (`SceneComponent.K2_GetComponentRotation` (`self.Camera`)) false false)
      (set `self.isJumping` false))))

(event `InputAction|Right`
  (params (Key :type "Key Structure"))
  (bind (_returnvalue_x _returnvalue_y _returnvalue_z) (`KismetMathLibrary.BreakVector` (`self.K2_GetActorLocation`)))
  (bind (_returnvalue_x_2 _returnvalue_y_2 _returnvalue_z_2) (`KismetMathLibrary.BreakVector` (`SceneComponent.K2_GetComponentLocation` (`self.Camera`))))
  (:`Pressed`
    (`AddComponent|NODE_AddAudioComponent-9`))
  (:`Released`
    (if (not (`self.isJumping`))
      (`SceneComponent.K2_SetRelativeRotation` (`self.Mesh`) (struct :`Yaw` 90.0) false false)
      (set `self.isJumping` true)
      (`self.Jump`)
      (`self.K2_SetActorRelativeLocation` (`KismetMathLibrary.MakeVector` _returnvalue_x (+ _returnvalue_y 215.0) _returnvalue_z))
      (`SceneComponent.K2_SetWorldLocationAndRotation` (`self.Camera`) (`KismetMathLibrary.MakeVector` _returnvalue_x_2 _returnvalue_y_2 _returnvalue_z_2) (`SceneComponent.K2_GetComponentRotation` (`self.Camera`)) false false)
      (set `self.isJumping` false))))

(event `InputAction|Down`
  (params (Key :type "Key Structure"))
  (bind (_returnvalue_x _returnvalue_y _returnvalue_z) (`KismetMathLibrary.BreakVector` (`self.K2_GetActorLocation`)))
  (bind (_returnvalue_x_2 _returnvalue_y_2 _returnvalue_z_2) (`KismetMathLibrary.BreakVector` (`SceneComponent.K2_GetComponentLocation` (`self.Camera`))))
  (:`Pressed`
    (`AddComponent|NODE_AddAudioComponent-7`))
  (:`Released`
    (if (not (`self.isJumping`))
      (`SceneComponent.K2_SetRelativeRotation` (`self.Mesh`) (struct :`Yaw` 540.0) false false)
      (set `self.isJumping` true)
      (`self.Jump`)
      (`self.K2_SetActorRelativeLocation` (`KismetMathLibrary.MakeVector` (+ _returnvalue_x -215.0) _returnvalue_y _returnvalue_z))
      (`SceneComponent.K2_SetWorldLocationAndRotation` (`self.Camera`) (`KismetMathLibrary.MakeVector` _returnvalue_x_2 _returnvalue_y_2 _returnvalue_z_2) (`SceneComponent.K2_GetComponentRotation` (`self.Camera`)) false false)
      (set `self.isJumping` false))))

(event `InputAction|Up`
  (params (Key :type "Key Structure"))
  (bind (_returnvalue_x _returnvalue_y _returnvalue_z) (`KismetMathLibrary.BreakVector` (`self.K2_GetActorLocation`)))
  (bind (_returnvalue_x_2 _returnvalue_y_2 _returnvalue_z_2) (`KismetMathLibrary.BreakVector` (`SceneComponent.K2_GetComponentLocation` (`self.Camera`))))
  (:`Pressed`
    (`AddComponent|NODE_AddAudioComponent-8`))
  (:`Released`
    (if (not (`self.isJumping`))
      (`SceneComponent.K2_SetRelativeRotation` :`self` (`self.Mesh`))
      (set `self.isJumping` true)
      (`self.Jump`)
      (`self.K2_SetActorRelativeLocation` (`KismetMathLibrary.MakeVector` (+ _returnvalue_x 215.0) _returnvalue_y _returnvalue_z))
      (`SceneComponent.K2_SetWorldLocationAndRotation` (`self.Camera`) (`KismetMathLibrary.MakeVector` _returnvalue_x_2 _returnvalue_y_2 _returnvalue_z_2) (`SceneComponent.K2_GetComponentRotation` (`self.Camera`)) false false)
      (set `self.isJumping` false))))

(fn `forward`)

(fn `moveLeft`)

(fn `set control rotation`)

(fn `UserConstructionScript`)