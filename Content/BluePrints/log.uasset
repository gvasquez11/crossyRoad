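; An actor Blueprint for a car that travels along the spline of a referenced track actor.
; On BeginPlay, if the car is active, it starts a timeline with play rate set from a duration and start time set from an offset.
; Each timeline update maps alpha to distance along the spline and sets the actor's world location and rotation to match that point.
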(event `self.ReceiveBeginPlay`
  (if (`self.activeCar`)
    (`self.MoveCar`)))

(event `MoveCar`
  (bind _returnvalue (`KismetMathLibrary.Lerp` 0.0 (`SplineComponent.GetSplineLength` (`/Game/BluePrints/track_.trackSpline` (`self.trackRef`))) (`self.Alpha`)))
  (`TimelineComponent.SetPlayRate` (`self.CarMover`) (/ 1.0 (`self.duration`)))
  (`TimelineComponent.SetNewTime` (`self.CarMover`) (`self.carStartOffset`))
  (bind (_direction _alpha) (`Timeline|CarMover`)
    (:`Update`
      (set `self.Alpha` _alpha)
      (`self.K2_SetActorLocationAndRotation` (`SplineComponent.GetLocationAtDistanceAlongSpline` (`/Game/BluePrints/track_.trackSpline` (`self.trackRef`)) _returnvalue "World") (`SplineComponent.GetRotationAtDistanceAlongSpline` (`/Game/BluePrints/track_.trackSpline` (`self.trackRef`)) _returnvalue "World")))))

(fn `UserConstructionScript`)